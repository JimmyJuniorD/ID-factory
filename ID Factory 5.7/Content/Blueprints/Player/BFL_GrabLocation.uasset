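; Blueprint function library that positions a grabbed item at the grabber's transform while accounting for static world geometry.
; A small sphere overlap-style trace at the End component checks whether the grab point touches WorldStatic objects.
; If it does, a second sphere trace from Start to End moves the item to the blocking hit location.
; The item always takes End's rotation and uses End's location when nothing blocks it.
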(fn SetGrabbedItemLocation
  (params (Start :type Scene%20Component%20Object%20Reference) (End :type Scene%20Component%20Object%20Reference) (Item :type Scene%20Component%20Object%20Reference))
  (bind _returnvalue (Transformation|GetWorldLocation End))
  ;[1 1 1] If Grabber is not Colliding Item transform remains Grabber transform
  (bind _returnvalue_2 (Collision|SphereTraceForObjects 0 _returnvalue _returnvalue 5.0 (Utilities|Array|MakeArray "ObjectTypeQuery1") false 0 "None"))
  (if _returnvalue_2
    ;[1 1 1] If Grabber Collides check for Collision between StartTraceLocation and GrabberLocation. If there is a Collision Set ItemLocation to HitLocation
    (bind _outhit (Collision|SphereTraceForObjects 0 (Transformation|GetWorldLocation Start) (Transformation|GetWorldLocation End) 5.0 (Utilities|Array|MakeArray "ObjectTypeQuery1") false 0 "None"))
    (Transformation|SetWorldLocationAndRotation Item (Math|Vector|SelectVector (.Location (Collision|BreakHitResult _outhit)) (Transformation|GetWorldLocation End) (.bBlockingHit (Collision|BreakHitResult _outhit))) (Transformation|GetWorldRotation End) false false)
    (else
      (Transformation|SetWorldLocationAndRotation Item (Transformation|GetWorldLocation End) (Transformation|GetWorldRotation End) false false))))