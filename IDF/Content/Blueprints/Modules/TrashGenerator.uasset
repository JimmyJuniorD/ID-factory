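; TrashGenerator is an actor Blueprint that periodically spawns trash and animates a lifter component.
; On BeginPlay it plays a timeline whose Height value is added to the Lifter's current world Z on every update, so the movement accumulates.
; It also starts a looping timer that spawns a RandomTrash actor at the SpawnLocation component every few seconds.
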(event Custom|SpawnTrash
  (Game|SpawnActorfromClass "/Game/Blueprints/Modules/randomTrash.randomTrash_C" (Math|Transform|MakeTransform (Transformation|GetWorldLocation (Variables|Default|GetSpawnLocation)) "0, 0, 0" "1.000000,1.000000,1.000000") "Undefined" "MultiplyWithRoot" 0 0))

(event EventTick
  (params (DeltaSeconds :type Float%20%28single-precision%29)))

(event EventBeginPlay
  (bind _lifter (Variables|Default|GetLifter))
  (Utilities|FlowControl|Sequence
    (:then_0
      (bind _height (Timeline|Timeline Play)
        (:Update
          (Transformation|SetWorldLocation _lifter (+ (Transformation|GetWorldLocation _lifter) (Math|Vector|MakeVector 0.0 0.0 _height)) false false))))
    (:then_1
      (Utilities|Time|SetTimerbyEvent (delegate Custom|SpawnTrash) 3.0 true))))

(fn ConstructionScript)